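; BP_ADS_MoveFX is an action Blueprint that shifts two referenced actors, Act1 and Act2, straight down when triggered.
; Its PerformAction event subtracts a fixed 1000-unit Z offset from each actor's current location and applies it instantly, without sweep.
; Each call lowers them further, with no interpolation or reset; BeginPlay, overlap and Tick are disabled stubs.
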(event `self.PerformAction`
  (bind _act2 (`self.Act2`))
  (bind _act1 (`self.Act1`))
  (`self.K2_SetActorLocation` _act1 (- (`self.K2_GetActorLocation` _act1) (0.0 0.0 1000.0)) false false)
  (`self.K2_SetActorLocation` _act2 (- (`self.K2_GetActorLocation` _act2) (0.0 0.0 1000.0)) false false))

(fn `UserConstructionScript`
  (`parent.UserConstructionScript`))