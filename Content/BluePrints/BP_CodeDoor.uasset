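; Code-locked door that swings open once a sequence of code parts, tied to linked post-its, matches its code.
; BeginPlay sets timeline speed, stores the mesh rotation and gives each post-it a reference to the door.
; AddCodePart concatenates parts; at the expected count, a match deactivates post-its, opens the door and triggers win dialogue, otherwise resetting with lose dialogue.
; Open runs once, lerping mesh rotation through a timeline.
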(event `self.ReceiveBeginPlay`
  (`|ExecutionSequence`
    (:`then_0`
      (`TimelineComponent.SetPlayRate` (`self.TimeLineDoor`) (`self.SpeedDoor`)))
    (:`then_1`
      (set `self.OriginalRotation` (`SceneComponent.RelativeRotation` (`self.StaticMesh`))))
    (:`then_2`
      (for _array_element (`self.PostItList`)
        (set `/Game/BluePrints/BP_I_PostIt.CodeDoor` self _array_element)))))

(event `Open`
  (`/Engine/EditorBlueprintResources/StandardMacros.DoOnce` false
    (:`Completed`
      (bind (_direction _newtrack_0) (`Timeline|TimeLineDoor`)
        (:`Update`
          (`SceneComponent.K2_SetRelativeRotation` (`self.StaticMesh`) (`KismetMathLibrary.RLerp` (`self.OriginalRotation`) (`self.NewRotation`) _newtrack_0) false false))
        (:`Finished`
          (`KismetSystemLibrary.PrintString` "Hello"))))))

(event `AddCodePart`
  (params (PartOfCode :type String))
  (`/Engine/EditorBlueprintResources/StandardMacros.IncrementInt` (`self.NumberOfTry`)
    (:`  `
      (set `self.TestingCode` (`KismetStringLibrary.Concat_StrStr` (`self.TestingCode`) PartOfCode))
      (if (== (`self.NumberOfPostItInCode`) (`self.NumberOfTry`))
        (if (`KismetStringLibrary.EqualEqual_StrStr` (`self.Code`) (`self.TestingCode`))
          (for _array_element (`self.PostItList`)
            (`/Game/BluePrints/BP_Interactable.SetActive` _array_element false)
            (`KismetSystemLibrary.Delay` 2.0)
            (`self.Open`)
            (`/Game/BluePrints/BP_ActorDoingSomething.PerformAction` (`self.WinDialogue`)))
          (else
            (set `self.NumberOfTry` 0)
            (set `self.TestingCode` "")
            (`KismetSystemLibrary.Delay` 2.0)
            (`/Game/BluePrints/BP_ActorDoingSomething.PerformAction` (`self.LoseDialogue`))))))))

(fn `UserConstructionScript`)