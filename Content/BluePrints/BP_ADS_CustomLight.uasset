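; BP_ADS_CustomLight is a point light actor that switches on or off once when its PerformAction event is called.
; PerformAction waits for DelayBeforePerforming, then sets the light's visibility to match the TurnOn flag.
; The construction script presets the light to the opposite state, so a light set to turn on starts hidden and vice versa.
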(event `self.PerformAction`
  (`KismetSystemLibrary.Delay` (`self.DelayBeforePerforming`))
  (if (`self.TurnOn`)
    (`SceneComponent.SetVisibility` (`self.PointLight`) true false)
    (else
      (`SceneComponent.SetVisibility` (`self.PointLight`) false false))))

(fn `UserConstructionScript`
  (if (`self.TurnOn`)
    (`SceneComponent.SetVisibility` (`self.PointLight`) false false)
    (else
      (`SceneComponent.SetVisibility` (`self.PointLight`) true false))))