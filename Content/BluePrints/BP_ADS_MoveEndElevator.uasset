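; BP_ADS_MoveEndElevator is an action Blueprint that repositions a referenced EndElevator actor.
; On BeginPlay it caches the elevator's location as OriginalPos, then shifts the elevator away from it along the Y axis.
; The PerformAction event snaps the elevator back to that original position with an instant, non-swept location set.
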(event `self.ReceiveBeginPlay`
  (bind _endelevator (`self.EndElevator`))
  (`parent.ReceiveBeginPlay`)
  (set `self.OriginalPos` (`self.K2_GetActorLocation` _endelevator))
  (`self.K2_SetActorLocation` _endelevator (- (`self.OriginalPos`) (0.0 -1000.0 0.0)) false false))

(event `self.PerformAction`
  (`self.K2_SetActorLocation` (`self.EndElevator`) (`self.OriginalPos`) false false))

(fn `UserConstructionScript`
  (`parent.UserConstructionScript`))