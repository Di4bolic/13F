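; Interactable door Blueprint that swings its mesh open on Interact, optionally consuming a key held by the controller.
; IsOpen guards Interact and is set before the key check, with no reset in this graph.
; OpenDoors deactivates itself, then a FlipFlop plays or reverses a speed-scaled timeline that lerps rotation from the BeginPlay original to NewRotation.
; The construction script applies the configurable handle mesh and location.
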(event `self.ReceiveBeginPlay`
  (`|ExecutionSequence`
    (:`then_0`
      (`TimelineComponent.SetPlayRate` (`self.TimelineDoor`) (`self.SpeedDoor`)))
    (:`then_1`
      (set `self.OriginalRotation` (`SceneComponent.K2_GetComponentRotation` (`self.StaticMesh`))))))

(event `self.Interact`
  (if (not (`self.IsOpen`))
    (set `self.IsOpen` true)
    (if (`self.NeedKey`)
      (bind _mycontroller (`/Game/BluePrints/BPFL_GetMyController.GetMyController`))
      (if (`/Game/BluePrints/BP_MyPlayerController.HasKey` _mycontroller)
        (set `/Game/BluePrints/BP_MyPlayerController.HasKey` false _mycontroller)
        (`self.OpenDoors` :!label _label)
        (`KismetSystemLibrary.PrintString` (`KismetStringLibrary.Conv_RotatorToString` (`self.OriginalRotation`)))
        (`KismetSystemLibrary.PrintString` (`KismetStringLibrary.Conv_RotatorToString` (`self.NewRotation`))))
      (else
        (goto _label)))))

(event `OpenDoors`
  (`self.SetActive` false)
  (`/Engine/EditorBlueprintResources/StandardMacros.FlipFlop`
    (:`A`
      (bind (_direction _newtrack_0) (`Timeline|TimelineDoor` :!label _label_2)
        (:`Update`
          (`SceneComponent.K2_SetWorldRotation` (`self.StaticMesh`) (`KismetMathLibrary.RLerp` (`self.OriginalRotation`) (`self.NewRotation`) _newtrack_0) false false))))
    (:`B`
      (goto _label_2 :!via `Reverse`))))

(fn `UserConstructionScript`
  (bind _handle (`self.Handle`))
  (`parent.UserConstructionScript`)
  (`StaticMeshComponent.SetStaticMesh` _handle (`self.HandleMesh`))
  (`SceneComponent.K2_SetRelativeLocation` _handle (`self.HandleLocation`) false false))