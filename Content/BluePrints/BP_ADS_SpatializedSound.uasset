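; BP_ADS_SpatializedSound is an actor that plays a spatialized sound at its own position when its PerformAction event fires.
; The event spawns the SoundToProduce sound at the default scene root's world location, using the shared SA_ForBasicObjects attenuation settings.
; BeginPlay, overlap and Tick are disabled stubs, and the construction script only calls the parent.
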(event `self.PerformAction`
  (`GameplayStatics.SpawnSoundAtLocation` (`self.SoundToProduce`) (`SceneComponent.K2_GetComponentLocation` (`self.DefaultSceneRoot`)) (struct) 1.0 1.0 0.0 "/Game/BluePrints/SA_ForBasicObjects.SA_ForBasicObjects" null))

(fn `UserConstructionScript`
  (`parent.UserConstructionScript`))