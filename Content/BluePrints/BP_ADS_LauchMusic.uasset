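; BP_ADS_LauchMusic is an action Blueprint that starts or stops music when its PerformAction event runs.
; It gets a controller through GetMyController and always stops the current music first.
; Unless the Stop flag is set, it then plays the Sound variable on that controller, so one asset serves both starting and silencing music.
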(event `self.PerformAction`
  (if (`self.Stop`)
    (bind _mycontroller (`/Game/BluePrints/BPFL_GetMyController.GetMyController`))
    (`/Game/BluePrints/BP_MyPlayerController.StopMusic` _mycontroller)
    (else
      (bind _mycontroller_2 (`/Game/BluePrints/BPFL_GetMyController.GetMyController`))
      (`/Game/BluePrints/BP_MyPlayerController.StopMusic` _mycontroller_2)
      (`/Game/BluePrints/BP_MyPlayerController.PlayMusic` _mycontroller_2 (`self.Sound`)))))

(fn `UserConstructionScript`
  (`parent.UserConstructionScript`))