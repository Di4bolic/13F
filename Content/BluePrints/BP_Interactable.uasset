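; BP_Interactable is an interactable actor that can trigger a linked dialogue once.
; Its Actions event calls Interact, an empty event in this graph, then runs Dialogue unless DialogueIsDone is already set.
; Dialogue sets that flag and calls PerformAction on LinkedDialogue if it is valid.
; The construction script applies the YourMesh variable to the static mesh component.
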(event `Interact`)

(event `Actions`
  (`self.Interact`)
  (if (not (`self.DialogueIsDone`))
    (`self.Dialogue`)))

(event `Dialogue`
  (bind _linkeddialogue (`self.LinkedDialogue`))
  (set `self.DialogueIsDone` true)
  (if (`KismetSystemLibrary.IsValid` _linkeddialogue)
    (`/Game/BluePrints/BP_ActorDoingSomething.PerformAction` _linkeddialogue)))

(fn `UserConstructionScript`
  (`StaticMeshComponent.SetStaticMesh` (`self.StaticMesh`) (`self.YourMesh`)))