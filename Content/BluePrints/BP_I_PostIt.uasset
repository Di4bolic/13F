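; Interactable post-it note that gives its code number to a linked code door and announces it through dialogue.
; On Interact it adds the number to CodeDoor, then picks an intro line based on whether the door's NumberOfTry equals one.
; It swaps that line into LinkedDialogue, plays it, then after a short delay restores and plays the original dialogue cached at BeginPlay.
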(event `self.ReceiveBeginPlay`
  (`parent.ReceiveBeginPlay`)
  (set `self.DialogueIsDone` true)
  (set `self.DialogueNumber` (`/Game/BluePrints/BP_ADS_Dialogue.Data` (`self.LinkedDialogue`))))

(event `self.Interact`
  (bind _linkeddialogue (`self.LinkedDialogue`))
  (bind _linkeddialogue_2 (`self.LinkedDialogue`))
  (bind _numberoftry (`/Game/BluePrints/BP_CodeDoor.NumberOfTry` (`self.CodeDoor`)))
  (`/Game/BluePrints/BP_CodeDoor.AddCodePArt` (`self.CodeDoor`) (`self.CodeNumber`))
  (if (== _numberoftry 1)
    (set `/Game/BluePrints/BP_ADS_Dialogue.Data` (`self.DialogueTry`) _linkeddialogue)
    (else
      (set `/Game/BluePrints/BP_ADS_Dialogue.Data` (`self.DialogueAnd`) (`self.LinkedDialogue`))))
  (`KismetSystemLibrary.PrintString` (`KismetStringLibrary.Conv_IntToString` _numberoftry))
  (`/Game/BluePrints/BP_ActorDoingSomething.PerformAction` _linkeddialogue)
  (`KismetSystemLibrary.Delay` 1.0)
  (set `/Game/BluePrints/BP_ADS_Dialogue.Data` (`self.DialogueNumber`) _linkeddialogue_2)
  (`/Game/BluePrints/BP_ActorDoingSomething.PerformAction` _linkeddialogue_2))

(fn `UserConstructionScript`
  (`parent.UserConstructionScript`))