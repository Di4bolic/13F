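; Interactable inspection pawn that blends the player's view to itself, then possesses it, and fires an optional linked dialogue action once.
; While possessed, holding left mouse rotates the Scene component from look and turn input when rotation is allowed.
; On release, it detaches the mesh, restores the Scene's rotation and reattaches, preserving the mesh's orientation while resetting the drag axes.
; Mesh and camera transform are configurable through the construction script.
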(event `self.ReceiveBeginPlay`)

(event `self.ReceiveActorBeginOverlap`
  (params (OtherActor :type "Actor Object Reference")))

(event `self.ReceiveTick`
  (params (DeltaSeconds :type "Float (single-precision)"))
  (bind _scene (`self.Scene`))
  (bind (_returnvalue_roll _returnvalue_pitch _returnvalue_yaw) (`KismetMathLibrary.BreakRotator` (`SceneComponent.K2_GetComponentRotation` _scene)))
  (if (`self.IsRotating`)
    (`SceneComponent.K2_SetWorldRotation` _scene (`KismetMathLibrary.MakeRotator` _returnvalue_roll (+ _returnvalue_pitch (* (`self.GetInputAxisValue`) 4.0)) (- _returnvalue_yaw (* (`self.GetInputAxisValue`) 4.0))) false false)))

(event `Actions`
  (`self.Interact`)
  (if (not (`self.DialogueDone`))
    (`self.Dialogue`)))

(event `Dialogue`
  (bind _linkeddialogue (`self.LinkedDialogue`))
  (set `self.DialogueDone` true)
  (if (`KismetSystemLibrary.IsValid` _linkeddialogue)
    (`/Game/BluePrints/BP_ActorDoingSomething.PerformAction` _linkeddialogue)))

(event `Interact`
  (bind _returnvalue (`GameplayStatics.GetPlayerController` 0))
  (bind _blendingtime (`self.BlendingTime`))
  (`PlayerController.SetViewTargetWithBlend` _returnvalue self _blendingtime "VTBlend_Linear" 0.0 false)
  (`KismetSystemLibrary.Delay` _blendingtime)
  (`Controller.Possess` _returnvalue self))

(event `Key|LeftMouseButton`
  (params (Key :type "Key Structure"))
  (bind _staticmesh (`self.StaticMesh`))
  (bind _scene (`self.Scene`))
  (:`Pressed`
    (if (`self.CanRotate`)
      (set `self.IsRotating` true)
      (set `self.OriginalRotation` (`SceneComponent.K2_GetComponentRotation` (`self.Scene`)))))
  (:`Released`
    (if (`self.CanRotate`)
      (set `self.IsRotating` false)
      (`SceneComponent.K2_DetachFromComponent` _staticmesh "KeepRelative" "KeepWorld" "KeepRelative" true)
      (`SceneComponent.K2_SetWorldRotation` _scene (`self.OriginalRotation`) false false)
      (`SceneComponent.K2_AttachToComponent` _staticmesh _scene "None" "KeepRelative" "KeepWorld" "KeepRelative" true))))

(event `SetActive`
  (params (IsActive :type Boolean))
  (set `self.IsActive` IsActive))

(fn `UserConstructionScript`
  (bind _camera (`self.Camera`))
  (`StaticMeshComponent.SetStaticMesh` (`self.StaticMesh`) (`self.YourMesh`))
  (`SceneComponent.K2_SetRelativeLocation` _camera (`self.CameraLocation`) false false)
  (`SceneComponent.K2_SetRelativeRotation` _camera (`self.CameraRotation`) false false))