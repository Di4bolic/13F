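; BP_ADS_LookAtWT is an action actor that runs a timed scripted sequence, taking control from the player to look at and approach set targets.
; PerformAction disables input and movement, enables look-at, sends the controller toward PlaceToGo, then crouches the player for a while.
; While Look is set, Tick turns control rotation toward PointToFocus.
; Fixed delays pace each step, after which the player stands and regains control.
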(event `self.ReceiveBeginPlay`
  (`parent.ReceiveBeginPlay`)
  (bind _player (`/Game/BluePrints/BPFL_GetPlayer.Get Player`))
  (set `self.Player` _player))

(event `self.ReceiveTick`
  (params (DeltaSeconds :type "Float (single-precision)"))
  (`parent.ReceiveTick` DeltaSeconds)
  (if (`self.Look`)
    (`Controller.SetControlRotation` (`self.MyController`) (`KismetMathLibrary.FindLookAtRotation` (`self.K2_GetActorLocation` (`self.Player`)) (`self.K2_GetActorLocation` (`self.PointToFocus`))))))

(event `self.PerformAction`
  (bind _mycontroller (`self.MyController`))
  (`self.DisableInput` (`self.Player`) _mycontroller)
  (set `/Game/BluePrints/BP_MyPlayerController.CanMove` false _mycontroller)
  (`KismetSystemLibrary.Delay` 0.5)
  (set `self.Look` true)
  (`KismetSystemLibrary.Delay` 0.5)
  (`AIBlueprintHelperLibrary.SimpleMoveToActor` (`self.MyController`) (`self.PlaceToGo`))
  (`KismetSystemLibrary.Delay` 2.5)
  (`Character.Crouch` (`self.Player`))
  (`KismetSystemLibrary.Delay` 8.0)
  (`Character.UnCrouch` (`self.Player`))
  (`self.EnableInput` (`self.Player`) null)
  (set `/Game/BluePrints/BP_MyPlayerController.CanMove` true (`self.MyController`))
  (set `self.Look` false))

(fn `UserConstructionScript`
  (`parent.UserConstructionScript`))