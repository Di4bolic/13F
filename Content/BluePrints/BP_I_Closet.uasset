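; Interactable closet that walks the player into position and triggers a quick-time event, unless that QTE is flagged as exited.
; Interact disables player movement and input, then uses SimpleMoveToActor toward a start actor.
; A delay loop polls until the player is close, pauses briefly, then calls the QTE's PerformAction.
; While interacting, Tick keeps control rotation aimed at a focus point until the QTE exit flag is set.
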(event `self.ReceiveBeginPlay`
  (`parent.ReceiveBeginPlay`)
  (bind _player (`/Game/BluePrints/BPFL_GetPlayer.Get Player`))
  (set `self.Player` _player)
  (bind _mycontroller (`/Game/BluePrints/BPFL_GetMyController.GetMyController`))
  (set `self.MyController` _mycontroller))

(event `self.ReceiveTick`
  (params (DeltaSeconds :type "Float (single-precision)"))
  (if (`/Game/BluePrints/BP_ADS_QTE.ExitQTE` (`self.QTE`))
    _
    (elif (`self.IsInteracting`)
      (`Controller.SetControlRotation` (`self.MyController`) (`KismetMathLibrary.FindLookAtRotation` (`self.K2_GetActorLocation` (`self.Player`)) (`SceneComponent.K2_GetComponentLocation` (`self.PointToFocus`)))))))

(event `self.Interact`
  (bind _mycontroller (`self.MyController`))
  (if (not (`/Game/BluePrints/BP_ADS_QTE.ExitQTE` (`self.QTE`)))
    (set `self.IsInteracting` true)
    (set `/Game/BluePrints/BP_MyPlayerController.CanMove` false _mycontroller)
    (`self.DisableInput` (`self.Player`) _mycontroller)
    (`AIBlueprintHelperLibrary.SimpleMoveToActor` (`self.MyController`) (`self.StartingPlayerPos`))
    (if (== (`self.K2_GetActorLocation` (`self.Player`)) (`self.K2_GetActorLocation` (`self.StartingPlayerPos`)) :`ErrorTolerance` 100.0) :!label _label
      (`KismetSystemLibrary.Delay` 0.5)
      (`/Game/BluePrints/BP_ActorDoingSomething.PerformAction` (`self.QTE`))
      (else
        (`KismetSystemLibrary.Delay` 0.1)
        (goto _label)))))

(fn `UserConstructionScript`
  (`parent.UserConstructionScript`))