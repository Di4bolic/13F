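; BP_Elevator_End is the ending elevator: its doors open at BeginPlay, close on the player and trigger the game's ending sequence.
; A FlipFlop plays or reverses a timeline that lerps both doors between cached offsets, setting DoorsOpen when finished.
; A capsule overlap, after confirming the first-person character remains inside, closes the doors and polls until shut.
; It then performs DialogueEnd's action and, after a delay, calls End on the controller.
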(event `self.ReceiveBeginPlay`
  (bind _relativelocation (`SceneComponent.RelativeLocation` (`self.DoorB`)))
  (`|ExecutionSequence`
    (:`then_0`
      (`TimelineComponent.SetPlayRate` (`self.TimelineDoors`) (`self.SpeedDoors`))
      (`self.Doors`))
    (:`then_1`
      (bind _output_get (set `self.LocationDoorAClosed` (`SceneComponent.RelativeLocation` (`self.DoorA`))))
      (set `self.LocationDoorBClosed` _relativelocation))
    (:`then_2`
      (set `self.LocationDoorAOpened` (+ _output_get (-100.0 0.0 0.0)))
      (set `self.LocationDoorBOpened` (+ _relativelocation (100.0 0.0 0.0))))))

(event `self.Box.OnComponentBeginOverlap`
  (params (OverlappedComponent :type "PrimitiveComponent Object Reference") (OtherActor :type "Actor Object Reference") (OtherComp :type "PrimitiveComponent Object Reference") (OtherBodyIndex :type Integer) (bFromSweep :type Boolean) (SweepResult :type "HitResult Structure (by ref)"))
  (cast `CapsuleComponent` OtherComp)
  (if (`self.DoorsOpen`)
    (`KismetSystemLibrary.Delay` 1.0)
    (for _array_element (`PrimitiveComponent.GetOverlappingActors` (`self.Box`) null)
      (cast `/Game/FirstPersonBP/Blueprints/FirstPersonCharacter` _array_element)
      (set `self.CanMove` true))
    (if (`self.CanMove`)
      (set `self.CanMove` false)
      (`self.Doors`)
      (if (`self.DoorsOpen`) :!label _label
        (`KismetSystemLibrary.Delay` 0.05)
        (goto _label)
        (else
          (`KismetSystemLibrary.Delay` 0.5)
          (`self.PerformAction` (`self.DialogueEnd`))
          (`KismetSystemLibrary.Delay` 13.0)
          (bind _mycontroller (`/Game/BluePrints/BPFL_GetMyController.GetMyController`))
          (`/Game/BluePrints/BP_MyPlayerController.End` _mycontroller))))))

(event `Doors`
  (bind _isa (`/Engine/EditorBlueprintResources/StandardMacros.FlipFlop`)
    (:`A`
      (bind (_direction _newtrack_0) (`Timeline|TimelineDoors` :!label _label_2)
        (:`Update`
          (`SceneComponent.K2_SetRelativeLocation` (`self.DoorA`) (`KismetMathLibrary.VLerp` (`self.LocationDoorAClosed`) (`self.LocationDoorAOpened`) _newtrack_0) false false)
          (`SceneComponent.K2_SetRelativeLocation` (`self.DoorB`) (`KismetMathLibrary.VLerp` (`self.LocationDoorBClosed`) (`self.LocationDoorBOpened`) _newtrack_0) false false))
        (:`Finished`
          (set `self.DoorsOpen` _isa))))
    (:`B`
      (goto _label_2 :!via `Reverse`))))

(fn `UserConstructionScript`)