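; Quick-time event actor, derived from a parent action class, that locks player input and movement until the QTE is won.
; PerformAction rebinds the "QTE" action mapping to its keyboard and gamepad keys at runtime and shows a radial-progress widget.
; It wins on one press or on spam presses that fill the bar against a timed Difficulty loop, optionally adjusted per press.
; Winning restores control after a short delay.
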(event `self.ReceiveBeginPlay`
  (bind _qteui (`self.QTEUI`))
  (`parent.ReceiveBeginPlay`)
  (bind _returnvalue (`|CreateWidget` "/Game/BluePrints/WBP_QTEInfinite.WBP_QTEInfinite_C" (`self.MyController`)))
  (bind _output_get (set `self.QTEUI` _returnvalue))
  (`UserWidget.AddToViewport` _output_get 0)
  (`Widget.SetVisibility` _qteui "Hidden")
  (`/Game/BluePrints/WBP_QTEInfinite.SetKeyQTEText` _qteui (`self.KeyKeyboard`)))

(event `self.PerformAction`
  (bind _mycontroller (`self.MyController`))
  (bind _player (`/Game/BluePrints/BPFL_GetPlayer.Get Player`))
  (`self.DisableInput` _player _mycontroller)
  (set `/Game/BluePrints/BP_MyPlayerController.CanMove` false _mycontroller)
  (`self.SwitchQTE`)
  (`self.BeginningActions`)
  (if (`self.JustOneClick`)
    (`self.BeginningOneClick` 0.0)
    (else
      (`self.BeginningSpamClick` 0.25))))

(event `SwitchQTE`
  (bind _returnvalue (`InputSettings.GetInputSettings`))
  (set `/Game/BluePrints/BP_MyPlayerController.QTE` self (cast `/Game/BluePrints/BP_MyPlayerController` (`GameplayStatics.GetPlayerController` 0) :!pure true))
  (for _array_element (`InputSettings.GetActionMappingByName` _returnvalue "QTE")
    (`InputSettings.RemoveActionMapping` _returnvalue _array_element false))
  (for _array_element_2 _
    (`InputSettings.RemoveActionMapping` _returnvalue _array_element_2 false))
  (`InputSettings.AddActionMapping` _returnvalue (make `InputActionKeyMapping` "QTE" false false false false (`self.KeyKeyboard`)) true)
  (`InputSettings.AddActionMapping` _returnvalue (make `InputActionKeyMapping` "QTE" false false false false (`self.KeyGamepad`)) true)
  (`Widget.SetVisibility` (`self.QTEUI`) "Visible"))

(event `BeginningOneClick`
  (params (Value :type "Float (double-precision)"))
  (bind _qteui (`self.QTEUI`))
  (bind _qteui_2 (`self.QTEUI`))
  (bind _output_get (set `/Game/BluePrints/WBP_QTEInfinite.RadialProgressBarValue` Value _qteui_2))
  (`MaterialInstanceDynamic.SetScalarParameterValue` (`/Game/BluePrints/WBP_QTEInfinite.MatInstance` _qteui_2) "Progress" _output_get)
  (bind _output_get_2 (set `/Game/BluePrints/WBP_QTEInfinite.RadialProgressBarValue` 1.1 _qteui))
  (`MaterialInstanceDynamic.SetScalarParameterValue` (`/Game/BluePrints/WBP_QTEInfinite.MatInstance` _qteui) "Progress" _output_get_2))

(event `BeginningSpamClick`
  (params (Value :type "Float (double-precision)"))
  (bind _qteui (`self.QTEUI`))
  (bind _qteui_2 (`self.QTEUI`))
  (bind _difficulty (`self.Difficulty`))
  (`self.BeginningOneClick` Value)
  (bind _output_get (set `/Game/BluePrints/WBP_QTEInfinite.RadialProgressBarValue` 0.2 _qteui_2))
  (`MaterialInstanceDynamic.SetScalarParameterValue` (`/Game/BluePrints/WBP_QTEInfinite.MatInstance` _qteui_2) "Progress" _output_get)
  (if (not (`self.Finished`)) :!label _label
    (`/Game/BluePrints/WBP_QTEInfinite.SetRadialProgressBar` _qteui _difficulty)
    (set `/Game/BluePrints/WBP_QTEInfinite.RadialProgressBarValue` (+ (`/Game/BluePrints/WBP_QTEInfinite.RadialProgressBarValue` _qteui) _difficulty) _qteui)
    (`KismetSystemLibrary.Delay` 0.06)
    (goto _label)))

(event `ReceiveInput`
  (bind _difficulty (`self.Difficulty`))
  (bind _qteui (`self.QTEUI`))
  (bind _maxdecreasedifficulty (`self.MaxDecreaseDifficulty`))
  (if (`self.JustOneClick`)
    (if (not (`self.Finished`)) :!label _label_2
      (`self.Win`)
      (`/Game/BluePrints/WBP_QTEInfinite.SetWin` (`self.QTEUI`))
      (`self.EndOfQTE`))
    (elif (not (`self.Finished`))
      (if (`self.RiseOfDifficulty`)
        (set `self.Difficulty` (- _difficulty (/ (`self.TimeBeforeFail`) (`self.RiseOfDifficultyValue`))))
        (if (<= _difficulty _maxdecreasedifficulty)
          (set `self.Difficulty` _maxdecreasedifficulty)))
      (`/Game/BluePrints/WBP_QTEInfinite.SetRadialProgressBar` _qteui 0.05)
      (if (>= (`/Game/BluePrints/WBP_QTEInfinite.RadialProgressBarValue` _qteui) 1.0)
        (set `/Game/BluePrints/WBP_QTEInfinite.RadialProgressBarValue` 1.1 _qteui)
        (goto _label_2)))))

(event `EndOfQTE`
  (bind _mycontroller (`self.MyController`))
  (set `self.Finished` true)
  (`KismetSystemLibrary.Delay` 1.5)
  (`Widget.SetVisibility` (`self.QTEUI`) "Hidden")
  (bind _player (`/Game/BluePrints/BPFL_GetPlayer.Get Player`))
  (`self.EnableInput` _player _mycontroller)
  (set `/Game/BluePrints/BP_MyPlayerController.CanMove` true _mycontroller)
  (set `self.ExitQTE` true))

(event `BeginningActions`
  (`KismetSystemLibrary.PrintString` "Beginning actions"))

(fn `UserConstructionScript`)