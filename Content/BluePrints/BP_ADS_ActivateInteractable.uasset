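; BP_ADS_ActivateInteractable is an action Blueprint that keeps a list of interactables switched off until its action is performed.
; On BeginPlay it runs the parent logic, then calls SetActive(false) on every entry in ListOfInteractables.
; The PerformAction event loops over the same list and calls SetActive(true), enabling them all at once.
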(event `self.ReceiveBeginPlay`
  (`parent.ReceiveBeginPlay`)
  (for _array_element (`self.ListOfInteractables`)
    (`/Game/BluePrints/BP_Interactable.SetActive` _array_element false)))

(event `self.PerformAction`
  (for _array_element (`self.ListOfInteractables`)
    (`/Game/BluePrints/BP_Interactable.SetActive` _array_element true)))

(fn `UserConstructionScript`
  (`parent.UserConstructionScript`))