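; BP_I_ElectricalSwitch is an interactable electrical switch that powers up a linked Elevator.
; On Interact it sets itself inactive, activates the Elevator and enables collision on a linked Trigger's box, which is disabled at BeginPlay.
; A timeline, with play rate set from Speed, lerps the switch mesh from its cached original rotation to NewRotation.
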(event `self.ReceiveBeginPlay`
  (`parent.ReceiveBeginPlay`)
  (`PrimitiveComponent.SetCollisionEnabled` (`/Game/BluePrints/BP_Trigger.Box` (`self.Trigger`)) "NoCollision")
  (set `self.OriginalRotation` (`SceneComponent.RelativeRotation` (`self.StaticMesh`)))
  (`TimelineComponent.SetPlayRate` (`self.TimelineRotation`) (`self.Speed`)))

(event `self.Interact`
  (`self.SetActive` false)
  (`/Game/BluePrints/BP_Elevator.Activate` (`self.Elevator`))
  (`PrimitiveComponent.SetCollisionEnabled` (`/Game/BluePrints/BP_Trigger.Box` (`self.Trigger`)) "QueryAndPhysics")
  (bind (_direction _newtrack_0) (`Timeline|TimelineRotation`)
    (:`Update`
      (`SceneComponent.K2_SetRelativeRotation` (`self.StaticMesh`) (`KismetMathLibrary.RLerp` (`self.OriginalRotation`) (`self.NewRotation`) _newtrack_0) false false))))

(fn `UserConstructionScript`
  (`parent.UserConstructionScript`))