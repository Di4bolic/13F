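; BP_ADS_ActivateTrigger is an action Blueprint that switches on a set of triggers when its action is performed.
; On BeginPlay it calls the parent, then disables collision on the Box of every entry in ListOfTriggers, so they start inactive.
; PerformAction loops over the same list and sets each Box to query and physics collision, with no path to disable them again.
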(event `self.ReceiveBeginPlay`
  (`parent.ReceiveBeginPlay`)
  (for _array_element (`self.ListOfTriggers`)
    (`PrimitiveComponent.SetCollisionEnabled` (`/Game/BluePrints/BP_Trigger.Box` _array_element) "NoCollision")))

(event `self.PerformAction`
  (for _array_element (`self.ListOfTriggers`)
    (`PrimitiveComponent.SetCollisionEnabled` (`/Game/BluePrints/BP_Trigger.Box` _array_element) "QueryAndPhysics")))

(fn `UserConstructionScript`
  (`parent.UserConstructionScript`))