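; First-person player controller that runs the intro logo and black-screen fades, gates movement, and handles interaction.
; A per-tick camera line trace highlights interactables; Use triggers them or, for interactable pawns, saves the view and frees the cursor.
; Pressing Use while possessing another pawn blends back and repossesses the character.
; It also forwards QTE input, teleports the player on a secret key code, and toggles two named post-process volumes.
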(event `self.ReceiveBeginPlay`
  (bind _walkingspeed (`self.WalkingSpeed`))
  (`|ExecutionSequence`
    (:`then_0`
      (bind _player (`/Game/BluePrints/BPFL_GetPlayer.Get Player`))
      (bind _output_get (set `self.ThePlayer` _player))
      (set `self.WalkingSpeed` 275.0)
      (bind _charactermovement (`Character.CharacterMovement` _output_get))
      (set `CharacterMovementComponent.MaxWalkSpeedCrouched` (/ _walkingspeed 2.0) _charactermovement)
      (set `CharacterMovementComponent.MaxWalkSpeed` _walkingspeed _charactermovement)
      (bind _returnvalue (`|CreateWidget` "/Game/BluePrints/WBP_MyUI.WBP_MyUI_C" self))
      (bind _output_get_2 (set `self.MyUI` _returnvalue))
      (`UserWidget.AddToViewport` _output_get_2 0)
      (bind _outactors (`GameplayStatics.GetAllActorsOfClass` "/Script/Engine.PostProcessVolume"))
      (for _array_element _outactors
        (if (`KismetStringLibrary.EqualEqual_StrStr` (`KismetSystemLibrary.GetDisplayName` _array_element) "PostProcessMathieu")
          (set `self.PostProcessMathieu` _array_element)
          (else
            (set `self.PostProcessEthan` _array_element)))))
    (:`then_1`
      (set `self.CanMove` false)
      (`self.DisableInput` (`self.ThePlayer`) null)
      (`KismetSystemLibrary.Delay` 1.0)
      (bind (_direction _newtrack_0) (`Timeline|TimelineLogoFade` :!via `PlayFromStart`)
        (:`Update`
          (`Widget.SetRenderOpacity` (`/Game/BluePrints/WBP_MyUI.Logo` (`self.MyUI`)) _newtrack_0))
        (:`Finished`
          (`KismetSystemLibrary.Delay` 2.0)
          (bind (_direction_2 _newtrack_0_2) (`Timeline|TimelineLogoFadeBis` :!via `ReverseFromEnd`)
            (:`Update`
              (`Widget.SetRenderOpacity` (`/Game/BluePrints/WBP_MyUI.Logo` (`self.MyUI`)) _newtrack_0_2))
            (:`Finished`
              (`KismetSystemLibrary.Delay` 1.0)
              (set `CharacterMovementComponent.GravityScale` 1.0 (`Character.CharacterMovement` (`self.ThePlayer`)))
              (bind (_direction_3 _newtrack_0_3) (`Timeline|TimelineBlackFade` :!via `ReverseFromEnd`)
                (:`Update`
                  (`Widget.SetRenderOpacity` (`/Game/BluePrints/WBP_MyUI.BlackScreen` (`self.MyUI`)) _newtrack_0_3))
                (:`Finished`
                  (`self.EnableInput` (`self.ThePlayer`) null)
                  (set `self.CanMove` true)
                  (set `PostProcessVolume.bEnabled` false (`self.PostProcessEthan`))
                  (set `PostProcessVolume.bEnabled` true (`self.PostProcessMathieu`)))))))))))

(event `InputAction|Use`
  (params (Key :type "Key Structure"))
  (bind _returnvalue (`GameplayStatics.GetPlayerController` 0))
  (bind _blendingtime (`self.BlendingTime`))
  (bind _originalcharacter (`self.OriginalCharacter`))
  (:`Pressed`
    (bind _asfirst_person_character (cast `/Game/FirstPersonBP/Blueprints/FirstPersonCharacter` (`GameplayStatics.GetPlayerPawn` 0))
      (:`then`
        (set `self.OriginalCharacter` _asfirst_person_character)
        (bind _firstpersoncamera (`/Game/FirstPersonBP/Blueprints/FirstPersonCharacter.FirstPersonCamera` _asfirst_person_character))
        (bind _returnvalue_2 (`SceneComponent.K2_GetComponentLocation` _firstpersoncamera))
        (bind _outhit (`KismetSystemLibrary.LineTraceSingle` _returnvalue_2 (+ _returnvalue_2 (* (`SceneComponent.GetForwardVector` _firstpersoncamera) (`self.visibilityDistance`))) "TraceTypeQuery1"))
        (if (not (`KismetSystemLibrary.IsValid` (`self.CurrentDialogue`)))
          (bind _asbp_interactable (cast `/Game/BluePrints/BP_Interactable` (`.HitActor` (`GameplayStatics.BreakHitResult` _outhit)))
            (:`then`
              (if (`/Game/BluePrints/BP_Interactable.IsActive` _asbp_interactable)
                (`/Game/BluePrints/BP_Interactable.Actions` _asbp_interactable)))
            (:`CastFailed`
              (bind _asbp_interactable_pawn (cast `/Game/BluePrints/BP_interactablePawn` (`.HitActor` (`GameplayStatics.BreakHitResult` _outhit))))
              (set `self.PlayerCameraInteractingRotation` (`self.GetControlRotation`))
              (`/Game/BluePrints/BP_interactablePawn.Actions` _asbp_interactable_pawn)
              (set `self.bShowMouseCursor` true)
              (`self.DisableInput` (`self.OriginalCharacter`) null)
              (set `self.CanMove` false)))))
      (:`CastFailed`
        (set `self.bShowMouseCursor` false)
        (`self.SetViewTargetWithBlend` _returnvalue _originalcharacter _blendingtime "VTBlend_Linear" 0.0 false)
        (`KismetSystemLibrary.Delay` _blendingtime)
        (`self.Possess` _returnvalue _originalcharacter)
        (`self.EnableInput` _originalcharacter null)
        (`self.SetControlRotation` (`self.PlayerCameraInteractingRotation`))
        (set `self.CanMove` true)))))

(event `self.ReceiveTick`
  (params (DeltaSeconds :type "Float (single-precision)"))
  (bind _asfirst_person_character (cast `/Game/FirstPersonBP/Blueprints/FirstPersonCharacter` (`GameplayStatics.GetPlayerPawn` 0)))
  (bind _firstpersoncamera (`/Game/FirstPersonBP/Blueprints/FirstPersonCharacter.FirstPersonCamera` _asfirst_person_character))
  (bind _returnvalue (`SceneComponent.K2_GetComponentLocation` _firstpersoncamera))
  (bind _outhit (`KismetSystemLibrary.LineTraceSingle` _returnvalue (+ _returnvalue (* (`SceneComponent.GetForwardVector` _firstpersoncamera) (`self.visibilityDistance`))) "TraceTypeQuery1"))
  (bind _asbp_interactable (cast `/Game/BluePrints/BP_Interactable` (`.HitActor` (`GameplayStatics.BreakHitResult` _outhit)))
    (:`then`
      (bind _output_get (set `self.LastInteractable` _asbp_interactable))
      (if (`/Game/BluePrints/BP_Interactable.IsActive` _output_get)
        (`/Game/BluePrints/BP_Interactable.SetNewRendering` _output_get true)
        (else
          (if (`KismetSystemLibrary.IsValid` (`self.LastInteractable`)) :!label _label
            (`/Game/BluePrints/BP_Interactable.SetNewRendering` (`self.LastInteractable`) false))
          (bind _asbp_interactable_pawn (cast `/Game/BluePrints/BP_interactablePawn` (`.HitActor` (`GameplayStatics.BreakHitResult` _outhit)))
            (:`then`
              (bind _output_get_2 (set `self.LastInteractablePawn` _asbp_interactable_pawn))
              (`PrimitiveComponent.SetRenderCustomDepth` (`/Game/BluePrints/BP_interactablePawn.StaticMesh` _output_get_2) true))
            (:`CastFailed`
              (if (`KismetSystemLibrary.IsValid` (`self.LastInteractablePawn`))
                (`PrimitiveComponent.SetRenderCustomDepth` (`/Game/BluePrints/BP_interactablePawn.StaticMesh` (`self.LastInteractablePawn`)) false)))))))
    (:`CastFailed`
      (goto _label))))

(event `InputAction|QTE`
  (params (Key :type "Key Structure"))
  (bind _qte (`self.QTE`))
  (:`Pressed`
    (if (`KismetSystemLibrary.IsValid` _qte)
      (`/Game/BluePrints/BP_ADS_QTEWidgetInGame.ReceiveInput` _qte)
      (else
        (`KismetSystemLibrary.PrintString` "Pas de QTE en cours")))))

(event `Key|AnyKey`
  (params (Key :type "Key Structure"))
  (:`Pressed`
    (`self.AddToCode` (`KismetTextLibrary.Conv_TextToString` (`KismetInputLibrary.Key_GetDisplayName` Key)))))

(event `InputAxis|MoveForward` :consume false :overrideparent false
  (params (AxisValue :type "Float (single-precision)"))
  (bind _theplayer (`self.ThePlayer`))
  (if (`self.CanMove`)
    (`Pawn.AddMovementInput` (`self.ThePlayer`) (select `bool` (`HeadMountedDisplayFunctionLibrary.IsHeadMountedDisplayEnabled`) :`false` (`self.GetActorForwardVector` _theplayer) :`true` (`SceneComponent.GetForwardVector` (`/Game/FirstPersonBP/Blueprints/FirstPersonCharacter.FirstPersonCamera` _theplayer))) AxisValue false)))

(event `InputAxis|MoveRight` :consume false :overrideparent false
  (params (AxisValue :type "Float (single-precision)"))
  (bind _theplayer (`self.ThePlayer`))
  (if (`self.CanMove`)
    (`Pawn.AddMovementInput` (`self.ThePlayer`) (select `bool` (`HeadMountedDisplayFunctionLibrary.IsHeadMountedDisplayEnabled`) :`false` (`self.GetActorRightVector` _theplayer) :`true` (`SceneComponent.GetRightVector` (`/Game/FirstPersonBP/Blueprints/FirstPersonCharacter.FirstPersonCamera` _theplayer))) AxisValue false)))

(event `AddToCode`
  (params (Key :type String))
  (bind _realcode (`self.RealCode`))
  (bind _returnvalue (`KismetArrayLibrary.Array_Add` (`self.Code`) Key))
  (if (`KismetStringLibrary.EqualEqual_StrStr` Key (`|GetArrayItem` _realcode _returnvalue))
    (if (== (`KismetArrayLibrary.Array_Length` _realcode) (`KismetArrayLibrary.Array_Length` (`self.Code`)))
      (`self.K2_SetActorLocation` (`self.ThePlayer`) (-3538.0 -3538.0 -3538.0) false false))
    (else
      (`KismetArrayLibrary.Array_Clear` (`self.Code`)))))

(event `SetPosProVol`
  (params (IsRed :type Boolean))
  (if IsRed
    (set `PostProcessVolume.bEnabled` true (`self.PostProcessEthan`))
    (set `PostProcessVolume.bEnabled` false (`self.PostProcessMathieu`))
    (else
      (set `PostProcessVolume.bEnabled` false (`self.PostProcessEthan`))
      (set `PostProcessVolume.bEnabled` true (`self.PostProcessMathieu`)))))

(fn `UserConstructionScript`)