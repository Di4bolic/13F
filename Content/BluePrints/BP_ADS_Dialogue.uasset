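; BP_ADS_Dialogue is an action Blueprint that plays a sequence of voiced dialogue lines with on-screen English text.
; PerformAction registers itself with the controller, toggles SetPosProVol, and walks Data table rows, playing each 2D sound and waiting its duration plus a per-row gap.
; After the last row it hides the text and clears the controller state.
; Stop silences the current sound, hides the text and blocks further lines.
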(event `self.ReceiveBeginPlay`
  (`parent.ReceiveBeginPlay`))

(event `self.PerformAction`
  (bind _mycontroller (`self.MyController`))
  (bind _mycontroller_2 (`self.MyController`))
  (set `/Game/BluePrints/BP_MyPlayerController.CurrentDialogue` self _mycontroller_2)
  (`/Game/BluePrints/BP_MyPlayerController.SetPosProVol` _mycontroller_2 true)
  (set `self.CurrentID` 0)
  (bind _outrownames (`DataTableFunctionLibrary.GetDataTableRowNames` (`self.Data`)))
  (if (< (`self.CurrentID`) (`KismetArrayLibrary.Array_Length` _outrownames)) :!label _label
    (if (not (`self.StopSound`))
      (`Widget.SetVisibility` (`/Game/BluePrints/WBP_MyUI.DialogueText` (`/Game/BluePrints/BP_MyPlayerController.MyUI` (`self.MyController`))) "Visible")
      (bind _returnvalue (`|GetDataTableRow` (`self.Data`) (`|GetArrayItem` _outrownames (`self.CurrentID`)))
        (:`then`
          (bind (_texteng _sound _soundfornextsound) (break `/Game/BluePrints/SDialogues` _returnvalue))
          (bind _returnvalue_2 (`GameplayStatics.SpawnSound2D` _sound 1.0 1.0 0.0 null))
          (set `self.CurrentSound` _returnvalue_2)
          (`TextBlock.SetText` (`/Game/BluePrints/WBP_MyUI.DialogueText` (`/Game/BluePrints/BP_MyPlayerController.MyUI` (`self.MyController`))) _texteng)
          (`KismetSystemLibrary.Delay` (+ (`SoundBase.Duration` _sound) _soundfornextsound))
          (`/Engine/EditorBlueprintResources/StandardMacros.IncrementInt` (`self.CurrentID`)
            (:`  `
              (goto _label))))))
    (else
      (set `self.CurrentID` 0)
      (`Widget.SetVisibility` (`/Game/BluePrints/WBP_MyUI.DialogueText` (`/Game/BluePrints/BP_MyPlayerController.MyUI` (`self.MyController`))) "Hidden")
      (set `/Game/BluePrints/BP_MyPlayerController.CurrentDialogue` null _mycontroller)
      (`/Game/BluePrints/BP_MyPlayerController.SetPosProVol` _mycontroller false))))

(event `Stop`
  (set `self.StopSound` true)
  (`AudioComponent.Stop` (`self.CurrentSound`))
  (`Widget.SetVisibility` (`/Game/BluePrints/WBP_MyUI.DialogueText` (`/Game/BluePrints/BP_MyPlayerController.MyUI` (`self.MyController`))) "Hidden"))

(fn `UserConstructionScript`
  (`parent.UserConstructionScript`))