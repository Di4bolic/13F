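; Box-shaped dissolve volume actor that feeds its transform to materials for a shape-based dissolve effect.
; The construction script writes the Cube component's world location, scale and forward, right and up axes into the PC_BoxDissolver Material Parameter Collection, describing an oriented box.
; Values are pushed only at construction, as the event graph has no runtime logic.
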(fn `UserConstructionScript`
  (bind _cube (`self.Cube`))
  (`KismetMaterialLibrary.SetVectorParameterValue` "/Game/VFX/Dissolve/PC_BoxDissolver.PC_BoxDissolver" "Location" (`KismetMathLibrary.Conv_VectorToLinearColor` (`SceneComponent.K2_GetComponentLocation` _cube)))
  (`KismetMaterialLibrary.SetVectorParameterValue` "/Game/VFX/Dissolve/PC_BoxDissolver.PC_BoxDissolver" "Bounds" (`KismetMathLibrary.Conv_VectorToLinearColor` (`SceneComponent.K2_GetComponentScale` _cube)))
  (`KismetMaterialLibrary.SetVectorParameterValue` "/Game/VFX/Dissolve/PC_BoxDissolver.PC_BoxDissolver" "X" (`KismetMathLibrary.Conv_VectorToLinearColor` (`SceneComponent.GetForwardVector` _cube)))
  (`KismetMaterialLibrary.SetVectorParameterValue` "/Game/VFX/Dissolve/PC_BoxDissolver.PC_BoxDissolver" "Y" (`KismetMathLibrary.Conv_VectorToLinearColor` (`SceneComponent.GetRightVector` _cube)))
  (`KismetMaterialLibrary.SetVectorParameterValue` "/Game/VFX/Dissolve/PC_BoxDissolver.PC_BoxDissolver" "Z" (`KismetMathLibrary.Conv_VectorToLinearColor` (`SceneComponent.GetUpVector` _cube))))