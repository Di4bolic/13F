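; BP_FlickeringLight1 is a VFX light actor with two rect lights that flicker at random intervals alongside a sparkle effect.
; Tick drives a chain of latent Delays, starting with a random whole-second wait that paces each burst.
; Each burst blinks both lights off and on twice in quick succession.
; NSSparkles toggles its active state once per burst, as the lights first come back on.
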(event `self.ReceiveTick`
  (params (DeltaSeconds :type "Float (single-precision)"))
  (bind _rectlight (`self.RectLight`))
  (bind _rectlight1 (`self.RectLight1`))
  (`KismetSystemLibrary.Delay` (`KismetMathLibrary.Conv_IntToDouble` (`KismetMathLibrary.RandomInteger` 10)))
  (`SceneComponent.SetVisibility` _rectlight false false)
  (`SceneComponent.SetVisibility` _rectlight1 false false)
  (`KismetSystemLibrary.Delay` 0.05)
  (`ActorComponent.ToggleActive` (`self.NS_Sparkles`))
  (`SceneComponent.SetVisibility` _rectlight true false)
  (`SceneComponent.SetVisibility` _rectlight1 true false)
  (`KismetSystemLibrary.Delay` 0.05)
  (`SceneComponent.SetVisibility` _rectlight false false)
  (`SceneComponent.SetVisibility` _rectlight1 false false)
  (`KismetSystemLibrary.Delay` 0.05)
  (`SceneComponent.SetVisibility` _rectlight true false)
  (`SceneComponent.SetVisibility` _rectlight1 true false))

(fn `UserConstructionScript`)