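; BP_CodeDoor is a code-locked door that rotates open once the correct sequence of post-it parts is entered.
; On BeginPlay it registers itself with each post-it in PostItList and derives the open rotation from the mesh's forward vector plus OpeningAngle.
; AddCodePart concatenates parts until the expected count, then opens after a delay on a match or resets.
; Open runs once, lerping the mesh rotation through a speed-adjustable timeline.
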(event `self.ReceiveBeginPlay`
  (`|ExecutionSequence`
    (:`then_0`
      (`TimelineComponent.SetPlayRate` (`self.TimeLineDoor`) (`self.SpeedDoor`)))
    (:`then_1`
      (bind _output_get (set `self.OriginalRotation` (`KismetMathLibrary.Conv_RotatorToVector` (`SceneComponent.RelativeRotation` (`self.StaticMesh`)))))
      (set `self.NewRotation` (+ _output_get (`self.OpeningAngle`))))
    (:`then_2`
      (for _array_element (`self.PostItList`)
        (set `/Game/MyBluePrints/BP_I_PostIt.CodeDoor` self _array_element)))))

(event `Open`
  (`/Engine/EditorBlueprintResources/StandardMacros.DoOnce` false
    (:`Completed`
      (bind (_direction _newtrack_0) (`Timeline|TimeLineDoor`)
        (:`Update`
          (`SceneComponent.K2_SetRelativeRotation` (`self.StaticMesh`) (`KismetMathLibrary.RLerp` (`KismetMathLibrary.Conv_VectorToRotator` (`self.OriginalRotation`)) (`KismetMathLibrary.Conv_VectorToRotator` (`self.NewRotation`)) _newtrack_0) false false))))))

(event `AddCodePart`
  (params (PartOfCode :type String))
  (`/Engine/EditorBlueprintResources/StandardMacros.IncrementInt` (`self.NumberOfTry`)
    (:`  `
      (set `self.TestingCode` (`KismetStringLibrary.Concat_StrStr` (`self.TestingCode`) PartOfCode))
      (if (== (`self.NumberOfPostItInCode`) (`self.NumberOfTry`))
        (if (`KismetStringLibrary.EqualEqual_StrStr` (`self.Code`) (`self.TestingCode`))
          (`KismetSystemLibrary.Delay` 2.0)
          (`self.Open`)
          (else
            (set `self.NumberOfTry` 0)
            (set `self.TestingCode` "")))))))

(fn `UserConstructionScript`)