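; BP_I_ElectricalSwitch is an interactable electrical switch that powers up an elevator.
; On BeginPlay it disables collision on a linked trigger's box, keeping that trigger inactive.
; When interacted with, it activates the referenced elevator and re-enables query and physics collision on the trigger box.
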(event `self.ReceiveBeginPlay`
  (`parent.ReceiveBeginPlay`)
  (`PrimitiveComponent.SetCollisionEnabled` (`/Game/MyBluePrints/BP_Trigger.Box` (`self.Trigger`)) "NoCollision"))

(event `self.Interact`
  (`/Game/MyBluePrints/BP_Elevator.Activate` (`self.Elevator`))
  (`PrimitiveComponent.SetCollisionEnabled` (`/Game/MyBluePrints/BP_Trigger.Box` (`self.Trigger`)) "QueryAndPhysics"))

(fn `UserConstructionScript`
  (`parent.UserConstructionScript`))