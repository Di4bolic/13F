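; First-person player controller that handles crouching, interaction, QTE input and the HUD interact prompt.
; A camera line trace each Tick shows the prompt over interactable actors or pawns, and Use repeats it to trigger them.
; Interacting with a pawn shows the cursor and disables character input; Use while controlling another pawn blends back and re-possesses the character.
; Crouch toggles on both press and release; QTE input forwards to the active QTE.
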(event `self.ReceiveBeginPlay`
  (bind _walkingspeed (`self.WalkingSpeed`))
  (bind _player (`/Game/MyBluePrints/BPFL_GetPlayer.Get Player`))
  (bind _output_get (set `self.ThePlayer` _player))
  (set `self.WalkingSpeed` 275.0)
  (bind _charactermovement (`Character.CharacterMovement` _output_get))
  (set `CharacterMovementComponent.MaxWalkSpeedCrouched` (/ _walkingspeed 2.0) _charactermovement)
  (set `CharacterMovementComponent.MaxWalkSpeed` _walkingspeed _charactermovement)
  (bind _returnvalue (`|CreateWidget` "/Game/MyBluePrints/WBP_MyUI.WBP_MyUI_C" self))
  (bind _output_get_2 (set `self.MyUI` _returnvalue))
  (`UserWidget.AddToViewport` _output_get_2 0)
  (`Widget.SetVisibility` (`/Game/MyBluePrints/WBP_MyUI.InteractText` (`self.MyUI`)) "Hidden"))

(event `InputAction|Crouch`
  (params (Key :type "Key Structure"))
  (bind _theplayer (`self.ThePlayer`))
  (:`Pressed`
    (if (`NavMovementComponent.IsCrouching` (`Character.CharacterMovement` _theplayer)) :!label _label
      (`Character.UnCrouch` _theplayer)
      (else
        (`Character.Crouch` _theplayer))))
  (:`Released`
    (goto _label)))

(event `InputAction|Use`
  (params (Key :type "Key Structure"))
  (bind _returnvalue (`GameplayStatics.GetPlayerController` 0))
  (bind _blendingtime (`self.BlendingTime`))
  (bind _originalcharacter (`self.OriginalCharacter`))
  (:`Pressed`
    (bind _asfirst_person_character (cast `/Game/FirstPersonBP/Blueprints/FirstPersonCharacter` (`GameplayStatics.GetPlayerPawn` 0))
      (:`then`
        (set `self.OriginalCharacter` _asfirst_person_character)
        (bind _firstpersoncamera (`/Game/FirstPersonBP/Blueprints/FirstPersonCharacter.FirstPersonCamera` _asfirst_person_character))
        (bind _returnvalue_2 (`SceneComponent.K2_GetComponentLocation` _firstpersoncamera))
        (bind _outhit (`KismetSystemLibrary.LineTraceSingle` _returnvalue_2 (+ _returnvalue_2 (* (`SceneComponent.GetForwardVector` _firstpersoncamera) (`self.visibilityDistance`))) "TraceTypeQuery1"))
        (bind _asbp_interactable (cast `/Game/MyBluePrints/BP_Interactable` (`.HitActor` (`GameplayStatics.BreakHitResult` _outhit)))
          (:`then`
            (`/Game/MyBluePrints/BP_Interactable.Interact` _asbp_interactable))
          (:`CastFailed`
            (bind _asbp_interactable_pawn (cast `/Game/MyBluePrints/BP_interactablePawn` (`.HitActor` (`GameplayStatics.BreakHitResult` _outhit))))
            (`/Game/MyBluePrints/BP_interactablePawn.Intercat` _asbp_interactable_pawn)
            (set `self.bShowMouseCursor` true)
            (`self.DisableInput` (`self.OriginalCharacter`) null))))
      (:`CastFailed`
        (set `self.bShowMouseCursor` false)
        (`self.SetViewTargetWithBlend` _returnvalue _originalcharacter _blendingtime "VTBlend_Linear" 0.0 false)
        (`KismetSystemLibrary.Delay` _blendingtime)
        (`self.Possess` _returnvalue _originalcharacter)
        (`self.EnableInput` _originalcharacter null)))))

(event `self.ReceiveTick`
  (params (DeltaSeconds :type "Float (single-precision)"))
  (bind _asfirst_person_character (cast `/Game/FirstPersonBP/Blueprints/FirstPersonCharacter` (`GameplayStatics.GetPlayerPawn` 0)))
  (bind _firstpersoncamera (`/Game/FirstPersonBP/Blueprints/FirstPersonCharacter.FirstPersonCamera` _asfirst_person_character))
  (bind _returnvalue (`SceneComponent.K2_GetComponentLocation` _firstpersoncamera))
  (bind _outhit (`KismetSystemLibrary.LineTraceSingle` _returnvalue (+ _returnvalue (* (`SceneComponent.GetForwardVector` _firstpersoncamera) (`self.visibilityDistance`))) "TraceTypeQuery1"))
  (cast `/Game/MyBluePrints/BP_Interactable` (`.HitActor` (`GameplayStatics.BreakHitResult` _outhit))
    (:`then`
      (`Widget.SetVisibility` (`/Game/MyBluePrints/WBP_MyUI.InteractText` (`self.MyUI`)) "Visible" :!label _label_2))
    (:`CastFailed`
      (cast `/Game/MyBluePrints/BP_interactablePawn` (`.HitActor` (`GameplayStatics.BreakHitResult` _outhit))
        (:`then`
          (goto _label_2))
        (:`CastFailed`
          (`Widget.SetVisibility` (`/Game/MyBluePrints/WBP_MyUI.InteractText` (`self.MyUI`)) "Hidden"))))))

(event `InputAction|QTE`
  (params (Key :type "Key Structure"))
  (bind _qte (`self.QTE`))
  (:`Pressed`
    (if (`KismetSystemLibrary.IsValid` _qte)
      (`/Game/MyBluePrints/BP_QTE.ReceiveInput` _qte)
      (else
        (`KismetSystemLibrary.PrintString` "Pas de QTE en cours")))))

(fn `UserConstructionScript`)