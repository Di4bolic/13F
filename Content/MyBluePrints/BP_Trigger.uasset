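; BP_Trigger is a placeable box trigger that calls PerformAction on each LinkedObject entry when any capsule component begins overlapping it.
; The HS flag blocks retriggering, either permanently with OneActivation or until DelayBeforeReactivation elapses; both are handled inside the loop over linked objects.
; The construction script sizes the box from exposed extents and raises it by its Z extent so its base sits at its parent's origin.
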(event `self.ReceiveBeginPlay`)

(event `self.Box.OnComponentBeginOverlap`
  (params (OverlappedComponent :type "PrimitiveComponent Object Reference") (OtherActor :type "Actor Object Reference") (OtherComp :type "PrimitiveComponent Object Reference") (OtherBodyIndex :type Integer) (bFromSweep :type Boolean) (SweepResult :type "HitResult Structure (by ref)"))
  (cast `CapsuleComponent` OtherComp)
  (if (not (`self.HS`))
    (for _array_element (`self.LinkedObject`)
      (`/Game/MyBluePrints/BP_ActorDoingSomething.PerformAction` _array_element)
      (if (`self.OneActivation`)
        (set `self.HS` true)
        (else
          (set `self.HS` true)
          (`KismetSystemLibrary.Delay` (`self.DelayBeforeReactivation`))
          (set `self.HS` false))))))

(fn `UserConstructionScript`
  (bind _box (`self.Box`))
  (bind _in_box_extent_z (`self.In Box Extent Z`))
  (`BoxComponent.SetBoxExtent` _box (`KismetMathLibrary.MakeVector` (`self.In Box Extent X`) (`self.In Box Extent Y`) _in_box_extent_z) true)
  (`SceneComponent.K2_SetRelativeLocation` _box (`KismetMathLibrary.MakeVector` 0.0 0.0 _in_box_extent_z) false false))