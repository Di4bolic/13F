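; Interactable door Blueprint that swings its static mesh open and closed on alternating Interact calls.
; BeginPlay sets the timeline play rate from SpeedDoor, stores the mesh's relative rotation as an X-axis direction vector, and adds OpeningAngle to derive the target.
; A FlipFlop plays or reverses the timeline, whose track lerps between rotators rebuilt from those two vectors.
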(event `self.ReceiveBeginPlay`
  (`|ExecutionSequence`
    (:`then_0`
      (`TimelineComponent.SetPlayRate` (`self.TimeLineDoor`) (`self.SpeedDoor`)))
    (:`then_1`
      (bind _output_get (set `self.OriginalRotation` (`KismetMathLibrary.Conv_RotatorToVector` (`SceneComponent.RelativeRotation` (`self.StaticMesh`)))))
      (set `self.NewRotation` (+ _output_get (`self.OpeningAngle`))))))

(event `self.Interact`
  (`/Engine/EditorBlueprintResources/StandardMacros.FlipFlop`
    (:`A`
      (bind (_direction _newtrack_0) (`Timeline|TimeLineDoor` :!label _label)
        (:`Update`
          (`SceneComponent.K2_SetRelativeRotation` (`self.StaticMesh`) (`KismetMathLibrary.RLerp` (`KismetMathLibrary.Conv_VectorToRotator` (`self.OriginalRotation`)) (`KismetMathLibrary.Conv_VectorToRotator` (`self.NewRotation`)) _newtrack_0) false false))))
    (:`B`
      (goto _label :!via `Reverse`))))

(fn `UserConstructionScript`)