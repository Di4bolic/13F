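; Elevator actor that carries the first-person character between PointA and PointB behind two sliding doors.
; A capsule overlap on the Box waits, checks for the player, then calls Doors and, after a pause, Move.
; Both use FlipFlops to play or reverse lerp timelines at SpeedElevator rate; delayed Doors calls follow travel updates.
; PerformAction also toggles the doors after a delay, while Activate is empty.
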(event `self.ReceiveBeginPlay`
  (bind _relativelocation (`SceneComponent.RelativeLocation` (`self.DoorB`)))
  (`|ExecutionSequence`
    (:`then_0`
      (`TimelineComponent.SetPlayRate` (`self.TimeLineElevator`) (`self.SpeedElevator`))
      (`TimelineComponent.SetPlayRate` (`self.TimelineDoors`) (`self.SpeedElevator`)))
    (:`then_1`
      (bind _output_get (set `self.LocationDoorAClosed` (`SceneComponent.RelativeLocation` (`self.DoorA`))))
      (set `self.LocationDoorBClosed` _relativelocation))
    (:`then_2`
      (set `self.LocationDoorAOpened` (+ _output_get (-100.0 0.0 0.0)))
      (set `self.LocationDoorBOpened` (+ _relativelocation (100.0 0.0 0.0))))))

(event `self.Box.OnComponentBeginOverlap`
  (params (OverlappedComponent :type "PrimitiveComponent Object Reference") (OtherActor :type "Actor Object Reference") (OtherComp :type "PrimitiveComponent Object Reference") (OtherBodyIndex :type Integer) (bFromSweep :type Boolean) (SweepResult :type "HitResult Structure (by ref)"))
  (cast `CapsuleComponent` OtherComp)
  (`KismetSystemLibrary.Delay` 2.0)
  (for _array_element (`PrimitiveComponent.GetOverlappingActors` (`self.Box`) null)
    (cast `/Game/FirstPersonBP/Blueprints/FirstPersonCharacter` _array_element)
    (`self.Doors`)
    (`KismetSystemLibrary.Delay` 1.0)
    (`self.Move`)))

(event `Move`
  (`/Engine/EditorBlueprintResources/StandardMacros.FlipFlop`
    (:`A`
      (bind (_direction _newtrack_0) (`Timeline|TimeLineElevator` :!label _label)
        (:`Update`
          (`self.K2_SetActorLocation` (`KismetMathLibrary.VLerp` (`self.K2_GetActorLocation` (`self.PointA`)) (`self.K2_GetActorLocation` (`self.PointB`)) _newtrack_0))
          (`KismetSystemLibrary.Delay` 4.0)
          (`self.Doors`))))
    (:`B`
      (goto _label :!via `Reverse`))))

(event `Doors`
  (`/Engine/EditorBlueprintResources/StandardMacros.FlipFlop`
    (:`A`
      (bind (_direction _newtrack_0) (`Timeline|TimelineDoors` :!label _label_2)
        (:`Update`
          (`SceneComponent.K2_SetRelativeLocation` (`self.DoorA`) (`KismetMathLibrary.VLerp` (`self.LocationDoorAClosed`) (`self.LocationDoorAOpened`) _newtrack_0) false false)
          (`SceneComponent.K2_SetRelativeLocation` (`self.DoorB`) (`KismetMathLibrary.VLerp` (`self.LocationDoorBClosed`) (`self.LocationDoorBOpened`) _newtrack_0) false false))))
    (:`B`
      (goto _label_2 :!via `Reverse`))))

(event `Activate`)

(event `self.PerformAction`
  (`KismetSystemLibrary.Delay` 2.0)
  (`self.Doors`))

(fn `UserConstructionScript`)