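; Quick-time event actor with a configurable mesh that demands a single press or button mashing before a timer expires.
; PerformAction registers it on the player controller, rebinds the "QTE" action mapping at runtime to its keys and shows WBP_QTE.
; A rate-scaled timeline drives the time bar and fails on expiry, while mash mode drains a radial bar that ReceiveInput refills.
; Win and Fail only print, and EndOfQTE hides the widget.
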(event `self.ReceiveBeginPlay`
  (bind _qteui (`self.QTEUI`))
  (bind _mycontroller (`/Game/MyBluePrints/BPFL_GetMyController.GetMyController`))
  (bind _output_get (set `self.MyController` _mycontroller))
  (bind _returnvalue (`|CreateWidget` "/Game/MyBluePrints/WBP_QTE.WBP_QTE_C" _output_get))
  (bind _output_get_2 (set `self.QTEUI` _returnvalue))
  (`UserWidget.AddToViewport` _output_get_2 0)
  (`Widget.SetVisibility` _qteui "Hidden")
  (`/Game/MyBluePrints/WBP_QTE.SetKeyQTEText` _qteui (`self.KeyKeyboard`))
  (`TimelineComponent.SetPlayRate` (`self.TimelineTime`) (/ 1.0 (`self.TimeBeforeFail`))))

(event `self.PerformAction`
  (`self.SwitchQTE`)
  (if (`self.JustOneClick`)
    (`self.BeginningOneClick`)
    (else
      (`self.BeginningSpamClick`))))

(event `SwitchQTE`
  (bind _returnvalue (`InputSettings.GetInputSettings`))
  (set `/Game/MyBluePrints/BP_MyPlayerController.QTE` self (cast `/Game/MyBluePrints/BP_MyPlayerController` (`GameplayStatics.GetPlayerController` 0) :!pure true))
  (for _array_element (`InputSettings.GetActionMappingByName` _returnvalue "QTE")
    (`InputSettings.RemoveActionMapping` _returnvalue _array_element false))
  (for _array_element_2 _
    (`InputSettings.RemoveActionMapping` _returnvalue _array_element_2 false))
  (`InputSettings.AddActionMapping` _returnvalue (make `InputActionKeyMapping` "QTE" false false false false (`self.KeyKeyboard`)) true)
  (`InputSettings.AddActionMapping` _returnvalue (make `InputActionKeyMapping` "QTE" false false false false (`self.KeyGamepad`)) true)
  (`Widget.SetVisibility` (`self.QTEUI`) "Visible"))

(event `BeginningOneClick`
  (bind (_direction _newtrack_0) (`Timeline|TimelineTime`)
    (:`Update`
      (`/Game/MyBluePrints/WBP_QTE.SetTimeBar` (`self.QTEUI`) _newtrack_0))
    (:`Finished`
      (if (not (`self.Finished`))
        (`self.Fail`)
        (`self.EndOfQTE`)))))

(event `BeginningSpamClick`
  (`self.BeginningOneClick`)
  (if (not (`self.Finished`)) :!label _label
    (`/Game/MyBluePrints/WBP_QTE.SetRadialProgressBar` (`self.QTEUI`) -0.003)
    (`KismetSystemLibrary.Delay` 0.05)
    (goto _label)))

(event `ReceiveInput`
  (bind _qteui (`self.QTEUI`))
  (if (`self.JustOneClick`)
    (if (not (`self.Finished`)) :!label _label_2
      (`self.Win`)
      (`self.EndOfQTE`))
    (else
      (`/Game/MyBluePrints/WBP_QTE.SetRadialProgressBar` _qteui 0.05)
      (if (>= (`/Game/MyBluePrints/WBP_QTE.RadialProgressBarValue` _qteui) 1.0)
        (set `/Game/MyBluePrints/WBP_QTE.RadialProgressBarValue` 1.1 _qteui)
        (goto _label_2)))))

(event `Fail`
  (`KismetSystemLibrary.PrintString` "Fail"))

(event `Win`
  (`KismetSystemLibrary.PrintString` "Win"))

(event `EndOfQTE`
  (set `self.Finished` true)
  (`Widget.SetVisibility` (`self.QTEUI`) "Hidden"))

(fn `UserConstructionScript`
  (`StaticMeshComponent.SetStaticMesh` (`self.StaticMesh`) (`self.YourMesh`)))